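; Player character with camera-relative movement, class-based melee combos and a modular body following the main mesh's pose.
; Attack plays montages from Combo data and buffers presses, with separate events to chain, lunge or reset.
; Hand overlaps during attacks damage BPI_Enemy actors.
; OnHit reduces GameInstance health, knocks back, plays a class hit reaction, resets the combo and updates the HUD bar, unless blocking, whose setters are unwired.
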(event `self.ReceiveBeginPlay`
  (`SkinnedMeshComponent.SetLeaderPoseComponent` (`self.Head`) (`self.Mesh`) false)
  (`SkinnedMeshComponent.SetLeaderPoseComponent` (`self.Hair`) (`self.Mesh`) false)
  (`SkinnedMeshComponent.SetLeaderPoseComponent` (`self.Glove`) (`self.Mesh`) false)
  (`SkinnedMeshComponent.SetLeaderPoseComponent` (`self.Shoe`) (`self.Mesh`) false)
  (`SkinnedMeshComponent.SetLeaderPoseComponent` (`self.Headgear`) (`self.Mesh`) false)
  (bind _asbp_gi (cast `/Game/Blueprint/Game/BP_GI` (`GameplayStatics.GetGameInstance`)))
  (set `self.GIRef` _asbp_gi)
  (bind _returnvalue (`|CreateWidget` "/Game/UI/WBP_UI.WBP_UI_C"))
  (bind _output_get (set `self.UIRef` _returnvalue))
  (`UserWidget.AddToViewport` _output_get 1)
  (set `self.HPBarRef` (`/Game/UI/WBP_UI.ProgressBar_79` (`self.UIRef`))))

(event `InputAxis|WalkForward`
  (params (AxisValue :type "Float (single-precision)"))
  (bind (_returnvalue_roll _returnvalue_pitch _returnvalue_yaw) (`KismetMathLibrary.BreakRotator` (`SceneComponent.K2_GetComponentRotation` (`self.Camera`))))
  (if (not (`self.isAttacking`))
    (`self.AddMovementInput` (`KismetMathLibrary.GetForwardVector` (`KismetMathLibrary.MakeRotator` 0.0 0.0 _returnvalue_yaw)) AxisValue)))

(event `InputAxis|WalkRight`
  (params (AxisValue :type "Float (single-precision)"))
  (bind (_returnvalue_roll _returnvalue_pitch _returnvalue_yaw) (`KismetMathLibrary.BreakRotator` (`SceneComponent.K2_GetComponentRotation` (`self.Camera`))))
  (if (not (`self.isAttacking`))
    (`self.AddMovementInput` (`KismetMathLibrary.GetRightVector` (`KismetMathLibrary.MakeRotator` 0.0 0.0 _returnvalue_yaw)) AxisValue)))

(event `InputAction|Block / Roll`
  (params (Key :type "Key Structure")))

(event `InputAction|Attack`
  (params (Key :type "Key Structure"))
  (bind (_combo_combos _combo_classref) (break `/Game/Data/Structs/S_DefaultCombos` (`self.Combo`)))
  (bind _output_montages (break `/Game/Data/Structs/S_Combo` (`|GetArrayItem` _combo_combos (`BlueprintMapLibrary.Map_Find` _combo_classref (`self.Class`)))))
  (:`Pressed`
    (if (`self.isAttacking`)
      (set `self.SaveAttack` true)
      (else
        (set `self.isAttacking` true)
        (`self.PlayAnimMontage` (`|GetArrayItem` _output_montages (`self.AttackCount`)) (`self.AttackSpeed`) :!label _label)
        (if (== (`self.AttackCount`) (`KismetArrayLibrary.Array_Length` _output_montages))
          (set `self.AttackCount` 0)
          (else
            (bind _result (`/Engine/EditorBlueprintResources/StandardMacros.IncrementInt` (`self.AttackCount`))
              (:`  `
                (`KismetSystemLibrary.PrintString` (`KismetStringLibrary.Conv_IntToString` _result))))))))))

(event `ComboAttackSave`
  (if (`self.SaveAttack`)
    (set `self.SaveAttack` false)
    (goto _label)))

(event `LaunchAnim`
  (bind (_combo_combos _combo_classref) (break `/Game/Data/Structs/S_DefaultCombos` (`self.Combo`)))
  (bind (_output_montages _output_force) (break `/Game/Data/Structs/S_Combo` (`|GetArrayItem` _combo_combos (`BlueprintMapLibrary.Map_Find` _combo_classref (`self.Class`)))))
  (bind _output (`|GetArrayItem` _output_force (- (`self.AttackCount`) 1)))
  (bind (_returnvalue_x _returnvalue_y) (`KismetMathLibrary.BreakVector` (* (`self.GetActorForwardVector`) _output)))
  ;[1 1 1] Launch
  (`KismetSystemLibrary.PrintString` (`KismetStringLibrary.Conv_DoubleToString` _output))
  (`self.LaunchCharacter` (`KismetMathLibrary.MakeVector` _returnvalue_x _returnvalue_y)))

(event `Restart Combo`
  (set `self.AttackCount` 0)
  (set `self.isAttacking` false)
  (set `self.SaveAttack` false))

(event `self.LeftHand.OnComponentBeginOverlap`
  (params (OverlappedComponent :type "PrimitiveComponent Object Reference") (OtherActor :type "Actor Object Reference") (OtherComp :type "PrimitiveComponent Object Reference") (OtherBodyIndex :type Integer) (bFromSweep :type Boolean) (SweepResult :type "HitResult Structure (by ref)"))
  ;[1 1 1] Sword Colission
  (`self.Hit` OtherActor))

(event `self.RightHand.OnComponentBeginOverlap`
  (params (OverlappedComponent :type "PrimitiveComponent Object Reference") (OtherActor :type "Actor Object Reference") (OtherComp :type "PrimitiveComponent Object Reference") (OtherBodyIndex :type Integer) (bFromSweep :type Boolean) (SweepResult :type "HitResult Structure (by ref)"))
  ;[1 1 1] Sword Colission
  (`self.Hit` OtherActor))

(event `Hit`
  (params (`Other Actor` :type "Actor Object Reference"))
  ;[1 1 1] Hit Func
  (if (`self.isAttacking`)
    (if (`KismetSystemLibrary.DoesImplementInterface` `Other Actor` "/Game/Blueprint/Interface/BPI_Enemy.BPI_Enemy_C")
      (message `/Game/Blueprint/Interface/BPI_Enemy.OnHit` `Other Actor` 2.0 (`self.K2_GetActorLocation`) (`self.GetActorForwardVector`)))))

(event `OnHit`
  (params (HitLoc :type "Vector Structure") (ForwardVec :type "Vector Structure") (Damage :type "Float (double-precision)"))
  (bind (_returnvalue_x _returnvalue_y) (`KismetMathLibrary.BreakVector` (* ForwardVec 1000.0)))
  (bind _giref (`self.GIRef`))
  (bind _giref_2 (`self.GIRef`))
  (if (not (`self.isBlocking`))
    (set `/Game/Blueprint/Game/BP_GI.Health` (- (`/Game/Blueprint/Game/BP_GI.Health` _giref) Damage) _giref)
    (`MovementComponent.StopMovementImmediately` (`self.CharacterMovement`))
    (`self.LaunchCharacter` (`KismetMathLibrary.MakeVector` _returnvalue_x _returnvalue_y))
    (`self.PlayAnimMontage` (select `/Game/Data/Enums/E_HeroClass` (`self.Class`) :`NewEnumerator0` "/Game/Animations/Montages/GetHit_SwordShieldAnim_Montage.GetHit_SwordShieldAnim_Montage" :`NewEnumerator6` "/Game/Animations/Montages/GetHit_DoubleSwordAnim_Montage.GetHit_DoubleSwordAnim_Montage" :`NewEnumerator1` "/Game/Animations/Montages/GetHit_SingleTwohandSwordAnim_Montage.GetHit_SingleTwohandSwordAnim_Montage" :`NewEnumerator2` "/Game/Animations/Montages/GetHit_BowAnim_Montage.GetHit_BowAnim_Montage" :`NewEnumerator3` "/Game/Animations/Montages/GetHit_MagicWandAnim_Montage.GetHit_MagicWandAnim_Montage" :!type "AnimMontage Object Reference"))
    (`self.Restart Combo`)
    (`ProgressBar.SetPercent` (`self.HPBarRef`) (/ (`/Game/Blueprint/Game/BP_GI.Health` _giref_2) (`/Game/Blueprint/Game/BP_GI.MaxHealth` _giref_2)))))

(fn `UserConstructionScript`)