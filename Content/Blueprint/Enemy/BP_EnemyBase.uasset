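; Base enemy character with modular body meshes, a health bar, and class-based melee combo attacks against BP_Player.
; Attack plays montages from per-class Combo data, buffering repeat requests for ComboAttackSave, while Launch adds forward lunge force.
; Hand overlaps during attacks damage the player.
; Unblocked hits reset the combo, reduce health, then either play a class reaction with knockback or destroy the enemy; block setters are unwired.
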(event `self.ReceiveBeginPlay`
  (set `CharacterMovementComponent.MaxWalkSpeed` (`self.MaxWalkSpeed`) (`self.CharacterMovement`))
  (`SkinnedMeshComponent.SetLeaderPoseComponent` (`self.Head`) (`self.Mesh`) false)
  (`SkinnedMeshComponent.SetLeaderPoseComponent` (`self.Hair`) (`self.Mesh`) false)
  (`SkinnedMeshComponent.SetLeaderPoseComponent` (`self.Glove`) (`self.Mesh`) false)
  (`SkinnedMeshComponent.SetLeaderPoseComponent` (`self.Shoe`) (`self.Mesh`) false)
  (`SkinnedMeshComponent.SetLeaderPoseComponent` (`self.Headgear`) (`self.Mesh`) false)
  (bind _aswbp_health_bar (cast `/Game/UI/WBP_HealthBar` (`WidgetComponent.GetUserWidgetObject` (`self.HealthBar`))))
  (bind _output_get (set `self.HPBar` _aswbp_health_bar))
  (`ProgressBar.SetPercent` (`/Game/UI/WBP_HealthBar.ProgressBar_25` _output_get) 1.0))

(event `/Game/Blueprint/Interface/IAttackable.OnHit`
  (params (Damage :type "Float (single-precision)") (ForwardVector :type "Vector Structure") (HitLoc :type "Vector Structure"))
  (bind (_returnvalue_x _returnvalue_y) (`KismetMathLibrary.BreakVector` (* HitLoc 1000.0)))
  (if (not (`self.isBlocking`))
    (`self.Restart Combo`)
    (bind _output_get (set `self.Health` (- (`self.Health`) Damage)))
    (`ProgressBar.SetPercent` (`/Game/UI/WBP_HealthBar.ProgressBar_25` (`self.HPBar`)) (/ _output_get (`self.MaxHealth`)))
    (if (> (`self.Health`) 0.0)
      (`self.PlayAnimMontage` (select `/Game/Data/Enums/E_HeroClass` (`self.Class`) :`NewEnumerator0` "/Game/Animations/Montages/GetHit_SwordShieldAnim_Montage.GetHit_SwordShieldAnim_Montage" :`NewEnumerator6` "/Game/Animations/Montages/GetHit_DoubleSwordAnim_Montage.GetHit_DoubleSwordAnim_Montage" :`NewEnumerator1` "/Game/Animations/Montages/GetHit_SingleTwohandSwordAnim_Montage.GetHit_SingleTwohandSwordAnim_Montage" :`NewEnumerator2` "/Game/Animations/Montages/GetHit_BowAnim_Montage.GetHit_BowAnim_Montage" :`NewEnumerator3` "/Game/Animations/Montages/GetHit_MagicWandAnim_Montage.GetHit_MagicWandAnim_Montage" :!type "AnimMontage Object Reference"))
      (`MovementComponent.StopMovementImmediately` (`self.CharacterMovement`))
      (`self.LaunchCharacter` (`KismetMathLibrary.MakeVector` _returnvalue_x _returnvalue_y))
      (`self.K2_SetActorRotation` (`KismetMathLibrary.FindLookAtRotation` (`SceneComponent.K2_GetComponentLocation` (`self.Mesh`)) ForwardVector) true)
      (else
        (`self.K2_DestroyActor`)))))

(event `Attack`
  (bind (_combo_combos _combo_classref) (break `/Game/Data/Structs/S_DefaultCombos` (`self.Combo`)))
  (bind _output_montages (break `/Game/Data/Structs/S_Combo` (`|GetArrayItem` _combo_combos (`BlueprintMapLibrary.Map_Find` _combo_classref (`self.Class`)))))
  ;[1 1 1] Attack + Attack Save
  (if (`self.isAttacking`)
    (set `self.SaveAttack` true)
    (else
      (set `self.isAttacking` true)
      (`self.PlayAnimMontage` (`|GetArrayItem` _output_montages (`self.AttackCount`)) (`self.AttackSpeed`) :!label _label)
      (if (== (`self.AttackCount`) 1)
        (set `self.AttackCount` 0)
        (else
          (`/Engine/EditorBlueprintResources/StandardMacros.IncrementInt` (`self.AttackCount`)))))))

(event `ComboAttackSave`
  ;[1 1 1] Attack + Attack Save
  (if (`self.SaveAttack`)
    (set `self.SaveAttack` false)
    (goto _label)))

(event `Restart Combo`
  ;[1 1 1] Restart the Combo
  (set `self.AttackCount` 0)
  (set `self.isAttacking` false)
  (set `self.SaveAttack` false))

(event `Launch`
  (bind (_combo_combos _combo_classref) (break `/Game/Data/Structs/S_DefaultCombos` (`self.Combo`)))
  (bind (_output_montages _output_force) (break `/Game/Data/Structs/S_Combo` (`|GetArrayItem` _combo_combos (`BlueprintMapLibrary.Map_Find` _combo_classref (`self.Class`)))))
  (bind (_returnvalue_x _returnvalue_y) (`KismetMathLibrary.BreakVector` (* (`self.GetActorForwardVector`) (`|GetArrayItem` _output_force (`self.AttackCount`)))))
  ;[1 1 1] Launch
  (`self.LaunchCharacter` (`KismetMathLibrary.MakeVector` _returnvalue_x _returnvalue_y)))

(event `self.RightHand.OnComponentBeginOverlap`
  (params (OverlappedComponent :type "PrimitiveComponent Object Reference") (OtherActor :type "Actor Object Reference") (OtherComp :type "PrimitiveComponent Object Reference") (OtherBodyIndex :type Integer) (bFromSweep :type Boolean) (SweepResult :type "HitResult Structure (by ref)"))
  (if (`self.isAttacking`)
    (`self.HitPlayer` OtherActor)))

(event `self.LeftHand.OnComponentBeginOverlap`
  (params (OverlappedComponent :type "PrimitiveComponent Object Reference") (OtherActor :type "Actor Object Reference") (OtherComp :type "PrimitiveComponent Object Reference") (OtherBodyIndex :type Integer) (bFromSweep :type Boolean) (SweepResult :type "HitResult Structure (by ref)"))
  (if (`self.isAttacking`)
    (`self.HitPlayer` OtherActor)))

(event `HitPlayer`
  (params (`Other Actor` :type "Actor Object Reference"))
  (bind _asbp_player (cast `/Game/Blueprint/Player/BP_Player` `Other Actor`))
  (`/Game/Blueprint/Player/BP_Player.OnHit` _asbp_player (`self.K2_GetActorLocation`) (`self.GetActorForwardVector`) 10.0))

(fn `UserConstructionScript`)